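; Vasija (jar) actor that can be picked up and dropped, and that collects piedra_Arbol_BP2 objects, logged as fruit ("fruta").
; Pickup disables the Cube's physics and attaches the root to the supplied component; Drop restores physics and detaches.
; When a piedra_Arbol_BP2 overlaps the Trigger, it loses Sphere gravity, attaches to the jar with relative rules and is flagged non-grabbable.
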(event OnComponentHit(Cube)
  (params (HitComponent :type Primitive%20Component%20Object%20Reference) (OtherActor :type Actor%20Object%20Reference) (OtherComp :type Primitive%20Component%20Object%20Reference) (NormalImpulse :type Vector :default "0, 0, 0") (Hit :type Hit%20Result%20Structure%20%28by%20ref%29)))

(event OnComponentBeginOverlap(trigger)
  (params (OverlappedComponent :type Primitive%20Component%20Object%20Reference) (OtherActor :type Actor%20Object%20Reference) (OtherComp :type Primitive%20Component%20Object%20Reference) (OtherBodyIndex :type Integer) (bFromSweep :type Boolean) (SweepResult :type Hit%20Result%20Structure%20%28by%20ref%29))
  (bind _aspiedra_arbol_bp2 (Utilities|Casting|CastTopiedra_Arbol_BP2 OtherActor))
  (Physics|SetEnableGravity (Variables|/Game/BluePrint/Arbol_BPs/piedra_Arbol_BP2.piedra_Arbol_BP2_C|GetSphere _aspiedra_arbol_bp2) false)
  (Transformation|AttachActorToActor _aspiedra_arbol_bp2 self "None" "KeepRelative" "KeepRelative" "KeepRelative" true)
  (Development|PrintString "fruta en vasija")
  (Variables|/Game/BluePrint/Arbol_BPs/piedra_Arbol_BP2.piedra_Arbol_BP2_C|Setagarrable _aspiedra_arbol_bp2 false))

(event EventBeginPlay)

(event Collision|EventActorBeginOverlap
  (params (OtherActor :type Actor%20Object%20Reference)))

(event EventTick
  (params (DeltaSeconds :type Float%20%28single-precision%29)))

(event EventDrop
  (Physics|SetSimulatePhysics (Variables|Default|GetCube) true)
  (Transformation|DetachFromActor "KeepWorld" "KeepWorld" "KeepWorld"))

(event EventPickup
  (params (AttachTo :type Scene%20Component%20Object%20Reference))
  (Physics|SetSimulatePhysics (Variables|Default|GetCube) false)
  (Transformation|AttachComponentToComponent (VehicleSound|GetRootComponent) AttachTo "None" "KeepWorld" "KeepWorld" "KeepWorld" false))

(fn ConstructionScript)