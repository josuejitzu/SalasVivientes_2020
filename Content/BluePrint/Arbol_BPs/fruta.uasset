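; Fruit actor in the tree minigame that drops when struck by a stone (piedra_Arbol_BP2).
; On a valid hit its Sphere starts simulating physics, then it asks FrutasSpawn_BP to spawn another fruit and a random VasijaPiedras_BP to spawn a stone.
; PuntoSpawn is set to None before its validity check, so the branch that clears the spawn point's Ocupado flag does not run.
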(event OnComponentHit(Sphere)
  (params (HitComponent :type Primitive%20Component%20Object%20Reference) (OtherActor :type Actor%20Object%20Reference) (OtherComp :type Primitive%20Component%20Object%20Reference) (NormalImpulse :type Vector :default "0, 0, 0") (Hit :type Hit%20Result%20Structure%20%28by%20ref%29))
  (Utilities|Casting|CastTopiedra_Arbol_BP2 OtherActor)
  (bind _output_get (Variables|Default|SetpuntoSpawn 0))
  (Utilities|IsValid (Variables|Default|GetpuntoSpawn)
    (:Is%20Valid
      (Variables|/Game/BluePrint/Arbol_BPs/puntoSpawn_Fruta.puntoSpawn_Fruta_C|Setocupado _output_get false))
    (:Is%20Not%20Valid
      _))
  (Physics|SetSimulatePhysics (Variables|Default|GetSphere) true)
  ;[1 1 1] Llama a FurtasSpawn_BP para que spawnee otra fruta
  (bind _returnvalue (Actor|GetActorOfClass "/Game/BluePrint/Arbol_BPs/FrutasSpawn_BP.FrutasSpawn_BP_C"))
  (Default|SpawnFruta _returnvalue)
  (bind _outactors (Actor|GetAllActorsOfClass "/Game/BluePrint/Arbol_BPs/vasijaPiedras_BP.vasijaPiedras_BP_C"))
  (Default|SpawnearPiedra (Utilities|Array|Get(acopy) _outactors (Math|Random|RandomInteger (Utilities|Array|Length _outactors)))))

(event EventBeginPlay)

(event Collision|EventActorBeginOverlap
  (params (OtherActor :type Actor%20Object%20Reference)))

(event EventTick
  (params (DeltaSeconds :type Float%20%28single-precision%29)))

(fn ConstructionScript)