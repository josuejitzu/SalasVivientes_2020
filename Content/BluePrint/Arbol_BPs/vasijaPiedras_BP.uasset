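; Stone vessel Blueprint that keeps itself stocked with Piedra_Arbol_BP2 stone actors.
; On BeginPlay it spawns an initial batch of scaled-down stones at an Arrow component's location, counting each one.
; When a stone ends overlap with the Box component, the count drops and, if below the maximum, a replacement spawns after a short delay.
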(event OnComponentEndOverlap(Box)
  (params (OverlappedComponent :type Primitive%20Component%20Object%20Reference) (OtherActor :type Actor%20Object%20Reference) (OtherComp :type Primitive%20Component%20Object%20Reference) (OtherBodyIndex :type Integer))
  (bind _cantidadpiedras (Variables|Default|GetcantidadPiedras))
  (Utilities|Casting|CastTopiedra_Arbol_BP2 OtherActor)
  (if (> _cantidadpiedras 0)
    (Math|Integer|DecrementInt _cantidadpiedras
      (:%20%20
        ;[1 1 1] Si una piedra deja la vasija, se spawnea una nueva
        (if (< (Variables|Default|GetcantidadPiedras) (Variables|Default|GetmaximoPiedras))
          (Utilities|FlowControl|Delay 2.0)
          (CallFunction|SpawnearPiedra))))))

(event Custom|SpawnearPiedra
  (Game|SpawnActorfromClass "/Game/BluePrint/Arbol_BPs/piedra_Arbol_BP2.piedra_Arbol_BP2_C" (Math|Transform|MakeTransform (.location (Transformation|GetWorldTransform (Variables|Default|GetArrow))) "0, 0, 0" "0.050000,0.050000,0.050000") "Undefined" 0 0)
  (Math|Integer|IncrementInt (Variables|Default|GetcantidadPiedras)
    (:%20%20
      (Development|PrintString "Piedra Spawneada"))))

(event EventBeginPlay
  (for _index (range 0 3)
    (CallFunction|SpawnearPiedra)))

(event Collision|EventActorBeginOverlap
  (params (OtherActor :type Actor%20Object%20Reference)))

(event EventTick
  (params (DeltaSeconds :type Float%20%28single-precision%29)))

(fn ConstructionScript)