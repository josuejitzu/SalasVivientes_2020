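; Puzzle manager Blueprint that tracks jigsaw (Rompecabezas) pieces placed in position and signals when the puzzle is complete.
; Each PiezaEnPosicion call increments a counter; once it reaches the hardcoded threshold, it prints a completion message.
; It then searches all Totem_Acertijo_BP actors and calls ActivarSimbolo on those matching this puzzle's riddle enum, lighting the totem symbol.
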(event Custom|PiezaEnPosicion
  (bind _piezasenposicion (Variables|Default|GetpiezasEnPosicion))
  ;[1 1 1] Lleva el conteo de cuantas piezas del rompecabezas hay en posicion
  (Math|Integer|IncrementInt _piezasenposicion
    (:%20%20
      (if (>= _piezasenposicion 2)
        (Development|PrintString "Rompecabezas completo")
        ;[1 1 1] Llama al Totem para que encienda el simbolo
        (bind _outactors (Actor|GetAllActorsOfClass "/Game/BluePrint/Totem_Acertijo_BP.Totem_Acertijo_BP_C"))
        (for _array_element _outactors
          (if (Utilities|Enum|Equal(Enum) (Variables|/Game/BluePrint/Totem_Acertijo_BP.Totem_Acertijo_BP_C|GetnombreAcertijo _array_element) "NewEnumerator2")
            (Default|ActivarSimbolo _array_element)))))))

(event EventBeginPlay)

(event Collision|EventActorBeginOverlap
  (params (OtherActor :type Actor%20Object%20Reference)))

(event EventTick
  (params (DeltaSeconds :type Float%20%28single-precision%29)))

(fn ConstructionScript)