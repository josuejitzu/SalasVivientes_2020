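; Target slot for a jigsaw puzzle (rompecabezas) that accepts one specific piece.
; On box overlap, it checks that the piece's name matches its own and that both actor rotations agree within a small tolerance.
; A match turns off gravity, attaches and snaps the piece to PosicionPieza, and makes it non-grabbable.
; It also notifies the first Rompecabezas actor in the level through PiezaEnPosicion.
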(event OnComponentBeginOverlap(Box)
  (params (OverlappedComponent :type Primitive%20Component%20Object%20Reference) (OtherActor :type Actor%20Object%20Reference) (OtherComp :type Primitive%20Component%20Object%20Reference) (OtherBodyIndex :type Integer) (bFromSweep :type Boolean) (SweepResult :type Hit%20Result%20Structure%20%28by%20ref%29))
  (bind _posicionpieza (Variables|Default|GetposicionPieza))
  (bind _aspieza_rompecabezas (Utilities|Casting|CastTopiezaRompecabezas OtherActor))
  (if (Utilities|Enum|Equal(Enum) (Variables|/Game/BluePrint/Rompecabezas_BPs/piezaRompecabezas.piezaRompecabezas_C|GetnombrePIeza _aspieza_rompecabezas) (Variables|Default|GetnombrePieza))
    (if (Math|Rotator|Equal(Rotator) (Transformation|GetActorRotation _aspieza_rompecabezas) (Transformation|GetActorRotation) 5.0)
      (Development|PrintString "Pieza colocada correctamente" true true "(R=0.000818,G=1.000000,B=0.000000,A=1.000000)" 5.0)
      ;[1 1 1] Colocar la pieza y deshabilitarla
      (Physics|SetEnableGravity (Variables|/Game/BluePrint/Rompecabezas_BPs/piezaRompecabezas.piezaRompecabezas_C|Getmesh _aspieza_rompecabezas) false)
      (Transformation|AttachComponentToComponent _aspieza_rompecabezas _posicionpieza "None" "KeepWorld" "SnapToTarget" "KeepRelative" true)
      (Transformation|SetActorLocation _aspieza_rompecabezas (Transformation|GetWorldLocation _posicionpieza) false false)
      (CallFunction|PiezaColocada)
      (Variables|/Game/BluePrint/Rompecabezas_BPs/piezaRompecabezas.piezaRompecabezas_C|Setagarrable _aspieza_rompecabezas false))))

(event Custom|PiezaColocada
  ;[1 1 1] Llama al afuncion en PuertaEscritos
  (bind _outactors (Actor|GetAllActorsOfClass "/Game/BluePrint/Rompecabezas_BPs/Rompecabezas.Rompecabezas_C"))
  (Default|PiezaEnPosicion (Utilities|Array|Get(acopy) _outactors)))

(event EventBeginPlay)

(event Collision|EventActorBeginOverlap
  (params (OtherActor :type Actor%20Object%20Reference)))

(event EventTick
  (params (DeltaSeconds :type Float%20%28single-precision%29)))

(fn ConstructionScript)