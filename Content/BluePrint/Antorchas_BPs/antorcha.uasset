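; Pickable torch actor with a fire particle and point light that ignites and burns out after a set time.
; Pickup and Drop toggle mesh physics and attachment.
; EncenderAntorcha fades the light in via timeline, then ConteoApagado waits and reverses a separate timeline; torches starting lit skip this through the already-lit guard.
; A trigger overlap with the fire pit also ignites it, though a comment marks this broken, with the pit calling directly.
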(event OnComponentBeginOverlap(trigger)
  (params (OverlappedComponent :type Primitive%20Component%20Object%20Reference) (OtherActor :type Actor%20Object%20Reference) (OtherComp :type Primitive%20Component%20Object%20Reference) (OtherBodyIndex :type Integer) (bFromSweep :type Boolean) (SweepResult :type Hit%20Result%20Structure%20%28by%20ref%29))
  ;[1 1 1] Trigger encendido de antorcha(NO esta funcionando, el pitFuego esta llamando por el momento a la funcion
  (if (== OtherActor "/Game/BluePrint/Antorchas_BPs/pitFuego_antorcha.pitFuego_antorcha")
    (CallFunction|EncenderAntorcha)
    (Development|PrintString "Antorcha Encendida")))

(event Custom|EncenderAntorcha
  ;[1 1 1] Encendido de Antorcha
  (if (Variables|Default|Getencendida)
    (Development|PrintString " Antorcha ya encedida,...descartando")
    (else
      (Development|PrintString "Encendiendo antorcha")
      (Components|Activation|SetActive (Variables|Default|GetParticleSystem) true false)
      (Variables|Default|Setencendida true)
      (bind _intensidad (Timeline|EncendidoLuz PlayFromStart)
        (:Update
          (Rendering|Components|Light|SetIntensity (Variables|Default|GetPointLight) _intensidad))
        (:Finished
          (CallFunction|ConteoApagado))))))

(event Custom|ConteoApagado
  ;[1 1 1] Apagado antorcha con tiempo
  (Utilities|FlowControl|Delay (Variables|Default|GettiempoEncendido))
  (Components|Activation|SetActive (Variables|Default|GetParticleSystem) false false)
  (Variables|Default|Setencendida false)
  (bind _intensidad (Timeline|Timeline_0 Reverse)
    (:Update
      (Rendering|Components|Light|SetIntensity (Variables|Default|GetPointLight) _intensidad))))

(event EventBeginPlay
  (if (Variables|Default|Getencendida)
    (CallFunction|EncenderAntorcha)
    (else
      (Components|Activation|SetActive (Variables|Default|GetParticleSystem) false false)
      (Rendering|Components|Light|SetIntensity (Variables|Default|GetPointLight) 0.0))))

(event Collision|EventActorBeginOverlap
  (params (OtherActor :type Actor%20Object%20Reference)))

(event EventTick
  (params (DeltaSeconds :type Float%20%28single-precision%29)))

(event EventDrop
  (Physics|SetSimulatePhysics (Variables|Default|GetTorch_mesh) true)
  (Transformation|DetachFromActor "KeepWorld" "KeepWorld" "KeepWorld"))

(event EventPickup
  (params (AttachTo :type Scene%20Component%20Object%20Reference))
  (Physics|SetSimulatePhysics (Variables|Default|GetTorch_mesh) false)
  (Transformation|AttachComponentToComponent (VehicleSound|GetRootComponent) AttachTo "None" "KeepWorld" "KeepWorld" "KeepWorld" false))

(fn ConstructionScript
  (bind _pointlight (Variables|Default|GetPointLight))
  (if (Variables|Default|Getencendida)
    (Rendering|Components|Light|SetIntensity _pointlight 5e+03)
    (else
      (Rendering|Components|Light|SetIntensity _pointlight 0.0))))