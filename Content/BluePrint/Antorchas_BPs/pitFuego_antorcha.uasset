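; A fire pit Blueprint that passes flame to and from torches (antorcha) through an overlap trigger.
; An unlit pit starts with its particle system and point light off.
; When a torch enters the trigger, a lit pit tells it to ignite, while an unlit pit lights itself if that torch is burning, turning on particles and light.
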(event OnComponentBeginOverlap(trigger)
  (params (OverlappedComponent :type Primitive%20Component%20Object%20Reference) (OtherActor :type Actor%20Object%20Reference) (OtherComp :type Primitive%20Component%20Object%20Reference) (OtherBodyIndex :type Integer) (bFromSweep :type Boolean) (SweepResult :type Hit%20Result%20Structure%20%28by%20ref%29))
  (if (Variables|Default|Getencendido)
    (CallFunction|EncenderAntorcha)
    (else
      ;[1 1 1] Si el pit no esta encendido esto se activa
      (bind _asantorcha (Utilities|Casting|CastToantorcha OtherActor))
      (if (Variables|/Game/BluePrint/Antorchas_BPs/antorcha.antorcha_C|Getencendida _asantorcha)
        (CallFunction|Encender)))))

(event Custom|Encender
  ;[1 1 1] Sistema de encendido de pit
  (Components|Activation|SetActive (Variables|Default|GetParticleSystem) true false)
  (Rendering|Components|Light|SetIntensity (Variables|Default|GetPointLight) 5e+03)
  (Variables|Default|Setencendido true))

(event Custom|EncenderAntorcha
  ;[1 1 1] Manda  a llamar a la anotrcha en Trigger para encenderal
  (bind _asantorcha (Utilities|Casting|CastToantorcha (stale OnComponentBeginOverlap(trigger) OtherActor)))
  (Default|EncenderAntorcha _asantorcha))

(event EventBeginPlay
  (if (not (Variables|Default|Getencendido))
    (Components|Activation|SetActive (Variables|Default|GetParticleSystem) false false)
    (Rendering|Components|Light|SetIntensity (Variables|Default|GetPointLight) 0.0)))

(event Collision|EventActorBeginOverlap
  (params (OtherActor :type Actor%20Object%20Reference)))

(event EventTick
  (params (DeltaSeconds :type Float%20%28single-precision%29)))

(fn ConstructionScript)