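; Torch (antorcha) spawner actor that creates torches at its own transform while keeping their count under a maximum.
; Pressing A calls SpawnAntorcha, which spawns and increments the counter, or prints a warning once the limit is reached.
; A torch leaving the Trigger component decrements the counter, freeing a slot, so the cap tracks end overlaps rather than destruction.
; A branch that would unlight the torch is disconnected.
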(event OnComponentEndOverlap(Trigger)
  (params (OverlappedComponent :type Primitive%20Component%20Object%20Reference) (OtherActor :type Actor%20Object%20Reference) (OtherComp :type Primitive%20Component%20Object%20Reference) (OtherBodyIndex :type Integer))
  (bind _cantidadantorchas (Variables|Default|GetcantidadAntorchas))
  ;[1 1 1] Se encarga de saber cuantas antorchas hay spawneadas
  (bind _asantorcha (Utilities|Casting|CastToantorcha OtherActor))
  (if (> _cantidadantorchas 0)
    (Math|Integer|DecrementInt _cantidadantorchas)))

(event Custom|SpawnAntorcha
  ;[1 1 1] Spawn de Antorchas
  (if (>= (Variables|Default|GetcantidadAntorchas) (Variables|Default|GetcantidadAntorchasMAX))
    (Development|PrintString "Limite de antorchas alcanzado")
    (else
      (Game|SpawnActorfromClass "/Game/BluePrint/Antorchas_BPs/antorcha.antorcha_C" (Transformation|GetActorTransform) "AdjustIfPossibleButAlwaysSpawn" 0 0)
      (Math|Integer|IncrementInt (Variables|Default|GetcantidadAntorchas)))))

(event EventBeginPlay)

(event Collision|EventActorBeginOverlap
  (params (OtherActor :type Actor%20Object%20Reference)))

(event EventTick
  (params (DeltaSeconds :type Float%20%28single-precision%29)))

(event Input|KeyboardEvents|A
  (params (Key :type Key%20Structure :default "None"))
  (:Pressed
    (CallFunction|SpawnAntorcha)))

(fn ConstructionScript)