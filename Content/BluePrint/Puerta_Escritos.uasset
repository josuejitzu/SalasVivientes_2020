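; Puerta_Escritos is a door actor (per its name) whose first symbol can light up through an animated emissive material.
; The construction script creates a dynamic instance of CuboApagado_MAT on Cube and stores it as CuboEmission.
; EncenderPrimerSimbolo, or the W key, plays Timeline_Emission, which drives the EmissionPotencia parameter.
; Two-piece puzzle logic that would trigger the symbol remains, but it is disconnected and marked unused.
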(event Custom|PiezaRompecabezas
  (params (nombrePieza :type String))
  ;[1 1 1] Lleva la logica de que piezas del Rompecabezas se colocaron EN DESUSO
)

(event Custom|EncenderPrimer%20Simbolo
  (Development|PrintString "Cambiando Emission")
  (bind _newtrack_0 (Timeline|Timeline_Emission Play)
    (:Update
      (Rendering|Material|SetScalarParameterValue (Variables|Default|GetCuboEmission) "EmissionPotencia" (.x _newtrack_0) :!class /Script/Engine.MaterialInstanceDynamic))))

(event EventBeginPlay)

(event Collision|EventActorBeginOverlap
  (params (OtherActor :type Actor%20Object%20Reference)))

(event EventTick
  (params (DeltaSeconds :type Float%20%28single-precision%29)))

(event Input|KeyboardEvents|W
  (params (Key :type Key%20Structure :default "None"))
  (:Pressed
    (Development|PrintString "Cambiando Emission")
    (bind _newtrack_0 (Timeline|Timeline_Emission Play)
      (:Update
        (Rendering|Material|SetScalarParameterValue (Variables|Default|GetCuboEmission) "EmissionPotencia" (.x _newtrack_0) :!class /Script/Engine.MaterialInstanceDynamic)))))

(fn ConstructionScript
  (bind _returnvalue (Rendering|Material|CreateDynamicMaterialInstance (Variables|Default|GetCube) 0 "/Game/MaterialesPrueba/CuboApagado_MAT.CuboApagado_MAT" "None" :!class /Script/Engine.PrimitiveComponent))
  (Variables|Default|SetCuboEmission _returnvalue))