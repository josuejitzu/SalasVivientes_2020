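; Cenote skull-puzzle trigger that checks whether a thrown skull is the correct one when it overlaps the Box.
; Any Craneo_BP that enters is destroyed; one flagged Correcto also prints a debug message and searches all Totem_Acertijo_BP actors.
; For each totem whose NombreAcertijo matches a fixed enum value, it turns on the first Cenote_Luz found and activates that totem's symbol.
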(event OnComponentBeginOverlap(Box)
  (params (OverlappedComponent :type Primitive%20Component%20Object%20Reference) (OtherActor :type Actor%20Object%20Reference) (OtherComp :type Primitive%20Component%20Object%20Reference) (OtherBodyIndex :type Integer) (bFromSweep :type Boolean) (SweepResult :type Hit%20Result%20Structure%20%28by%20ref%29))
  ;[1 1 1] Checa si el craneo que se lanzo es el correcto o no
  (bind _ascraneo_bp (Utilities|Casting|CastToCraneo_BP OtherActor))
  (if (Variables|/Game/BluePrint/Cenote_BPs/Craneo_BP.Craneo_BP_C|Getcorrecto _ascraneo_bp)
    (Development|PrintString "Calavera Correcta")
    (Actor|DestroyActor _ascraneo_bp)
    ;[1 1 1] Si es correcto el craneo se busca el Totem correspondiente y se pide que se encienda su simbolo
    (bind _outactors (Actor|GetAllActorsOfClass "/Game/BluePrint/Totem_Acertijo_BP.Totem_Acertijo_BP_C"))
    (for _array_element _outactors
      (if (Utilities|Enum|Equal(Enum) (Variables|/Game/BluePrint/Totem_Acertijo_BP.Totem_Acertijo_BP_C|GetnombreAcertijo _array_element) "NewEnumerator0")
        (bind _outactors_2 (Actor|GetAllActorsOfClass "/Game/BluePrint/Cenote_BPs/Cenote_Luz.Cenote_Luz_C"))
        (Default|EncenderLuzCenote (Utilities|Array|Get(acopy) _outactors_2))
        (Default|ActivarSimbolo _array_element)))
    (else
      (Actor|DestroyActor _ascraneo_bp))))

(event EventBeginPlay)

(event Collision|EventActorBeginOverlap
  (params (OtherActor :type Actor%20Object%20Reference)))

(event EventTick
  (params (DeltaSeconds :type Float%20%28single-precision%29)))

(fn ConstructionScript)