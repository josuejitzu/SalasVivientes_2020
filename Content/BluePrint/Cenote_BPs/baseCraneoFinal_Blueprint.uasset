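; Final skull base for a cenote puzzle that tracks how many skulls have been placed correctly.
; Each CraneoColocado event increments CraneosCorrectos, and the third prints a completion message and gathers every Craneo_BP actor.
; A loop over those actors makes the Craneo component of those flagged Correcto visible after a short Delay.
; The Delay sits inside the loop body, so it does not wait separately for each skull.
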(event Custom|CraneoColocado
  (bind _craneoscorrectos (Variables|Default|GetcraneosCorrectos))
  (Math|Integer|IncrementInt _craneoscorrectos
    (:%20%20
      (if (== _craneoscorrectos 3)
        (Development|PrintString "Todos los craneos colocados")
        (bind _outactors (Actor|GetAllActorsOfClass "/Game/BluePrint/Cenote_BPs/Craneo_BP.Craneo_BP_C"))
        (for _array_element _outactors
          (if (Variables|/Game/BluePrint/Cenote_BPs/Craneo_BP.Craneo_BP_C|Getcorrecto _array_element)
            (Utilities|FlowControl|Delay 2.0)
            (Rendering|SetVisibility (Variables|/Game/BluePrint/Cenote_BPs/Craneo_BP.Craneo_BP_C|GetCraneo _array_element) true false)))))))

(event EventBeginPlay)

(event Collision|EventActorBeginOverlap
  (params (OtherActor :type Actor%20Object%20Reference)))

(event EventTick
  (params (DeltaSeconds :type Float%20%28single-precision%29)))

(fn ConstructionScript)