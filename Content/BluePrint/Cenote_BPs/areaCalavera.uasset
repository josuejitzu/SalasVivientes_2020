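; Skull placement zone for the cenote puzzle that accepts only the skull whose number matches its own.
; On trigger overlap with the matching Craneo_BP, it makes that skull non-grabbable and lights its symbol.
; A timeline drives the EmissionPotencia parameter on a dynamic material created in the construction script.
; Each timeline update, not just completion, also calls CraneoColocado on the first BaseCraneoFinal_Blueprint found in the level.
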(event OnComponentBeginOverlap(trigger)
  (params (OverlappedComponent :type Primitive%20Component%20Object%20Reference) (OtherActor :type Actor%20Object%20Reference) (OtherComp :type Primitive%20Component%20Object%20Reference) (OtherBodyIndex :type Integer) (bFromSweep :type Boolean) (SweepResult :type Hit%20Result%20Structure%20%28by%20ref%29))
  (bind _ascraneo_bp (Utilities|Casting|CastToCraneo_BP OtherActor))
  (if (== (Variables|Default|GetnumeroCalavera) (Variables|/Game/BluePrint/Cenote_BPs/Craneo_BP.Craneo_BP_C|GetnumeroCraneo _ascraneo_bp))
    (Variables|/Game/BluePrint/Cenote_BPs/Craneo_BP.Craneo_BP_C|Setagarrable _ascraneo_bp false)
    (Development|PrintString "Craneo Correcto" true true "(R=0.000000,G=0.660000,B=1.000000,A=1.000000)" 3.0)
    (CallFunction|EncenderSimbolo)))

(event Custom|EncenderSimbolo
  (Development|PrintString "Cambiando Emission")
  (bind _newtrack_0 (Timeline|Timeline_0 Play)
    (:Update
      (Rendering|Material|SetScalarParameterValue (Variables|Default|GetestanciaMaterial) "EmissionPotencia" (.x _newtrack_0) :!class /Script/Engine.MaterialInstanceDynamic)
      (bind _outactors (Actor|GetAllActorsOfClass "/Game/BluePrint/Cenote_BPs/baseCraneoFinal_Blueprint.baseCraneoFinal_Blueprint_C"))
      (Default|CraneoColocado (Utilities|Array|Get(acopy) _outactors)))))

(event EventBeginPlay)

(event Collision|EventActorBeginOverlap
  (params (OtherActor :type Actor%20Object%20Reference)))

(event EventTick
  (params (DeltaSeconds :type Float%20%28single-precision%29)))

(fn ConstructionScript
  (bind _returnvalue (Rendering|Material|CreateDynamicMaterialInstance (Variables|Default|Getsimboloencendido) 0 "/Game/MaterialesPrueba/CuboApagado_MAT.CuboApagado_MAT" "None" :!class /Script/Engine.PrimitiveComponent))
  (Variables|Default|SetestanciaMaterial _returnvalue))