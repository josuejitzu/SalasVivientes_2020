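; Grabbable skull (Craneo) actor from the Cenote blueprints that can be picked up and dropped.
; Pickup checks the Agarrable flag, then turns off the skull's physics and attaches the actor's root to the supplied component, keeping world transform.
; Drop re-enables physics and detaches the actor.
; A branch that would hide the skull when Correcto is true is unconnected and never runs.
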(event EventBeginPlay)

(event Collision|EventActorBeginOverlap
  (params (OtherActor :type Actor%20Object%20Reference)))

(event EventTick
  (params (DeltaSeconds :type Float%20%28single-precision%29)))

(event EventDrop
  (Physics|SetSimulatePhysics (Variables|Default|GetCraneo) true)
  (Transformation|DetachFromActor "KeepWorld" "KeepWorld" "KeepWorld"))

(event EventPickup
  (params (AttachTo :type Scene%20Component%20Object%20Reference))
  (if (Variables|Default|Getagarrable)
    (Physics|SetSimulatePhysics (Variables|Default|GetCraneo) false)
    (Transformation|AttachComponentToComponent (VehicleSound|GetRootComponent) AttachTo "None" "KeepWorld" "KeepWorld" "KeepWorld" false)))

(fn ConstructionScript)